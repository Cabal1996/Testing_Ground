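; Projectile Blueprint that leaves a plasma-hole decal where it hits.
; On projectile hit, it attaches the decal to the hit component and bone, aligned to the impact normal with random roll and size.
; The decal is set to a small fade screen size and a long timed fade-out.
; The generic Hit event only prints a debug string, while point damage and self-destruction logic is unconnected.
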(event Collision|EventHit
  (params (MyComp :type Primitive%20Component%20Object%20Reference) (Other :type Actor%20Object%20Reference) (OtherComp :type Primitive%20Component%20Object%20Reference) (bSelfMoved :type Boolean) (HitLocation :type Vector :default "0, 0, 0") (HitNormal :type Vector :default "0, 0, 0") (NormalImpulse :type Vector :default "0, 0, 0") (Hit :type Hit%20Result%20Structure%20%28by%20ref%29))
  (Development|PrintString "Hello"))

(event EventOnProjectileHit
  (bind _returnvalue (Class|Projectile|GetImpactNormal))
  (bind _returnvalue_2 (Math|Random|RandomFloatinRange 4.0 6.0))
  (bind _returnvalue_3 (Math|Rotator|MakeRotfromX _returnvalue))
  (bind _returnvalue_4 (Class|GameplayStatics|SpawnDecalAttached "/Game/Weapon/Decal/D_PlasmaHole.D_PlasmaHole" (Math|Vector|MakeVector 1e+01 _returnvalue_2 _returnvalue_2) (Class|Projectile|GetComponentOfHit) (Class|Projectile|GetBoneName) (Class|Projectile|GetImpactPoint) (Math|Rotator|MakeRotator (+ (.roll _returnvalue_3) (Math|Random|RandomFloatinRange 0.0 3.6e+02)) (+ (.pitch _returnvalue_3) 1.8e+02) (.yaw _returnvalue_3)) "KeepWorldPosition" 0.0001))
  (Utilities|IsValid _returnvalue_4
    (:Is%20Valid
      (Rendering|Components|Decal|SetFadeScreenSize _returnvalue_4 0.0025)
      (Rendering|Components|Decal|SetFadeOut _returnvalue_4 0.0 4e+01 false))))

(fn ConstructionScript)
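; BP_Container is a terrain prop that randomly spawns one pickup or none on BeginPlay: shotgun ammo box, ammo chest, or Armor30.
; Chained range checks each roll a fresh 1–100 number, so later items have lower odds and the container often stays empty.
; The chosen pickup spawns at the Arrow component, attaches to the container and takes the Arrow's relative location.
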(event EventBeginPlay
  (bind _returnvalue (Math|Random|RandomIntegerinRange 1 100))
  (bind _arrow (Variables|Default|GetArrow))
  (bind _arrow_2 (Variables|Default|GetArrow))
  (bind _arrow_3 (Variables|Default|GetArrow))
  (if (Math|Integer|InRange(Integer) _returnvalue 1 25)
    (bind _returnvalue_2 (Game|SpawnActorfromClass "/Game/Terrain/Pickups/AmmoBoxShodgun_BP.AmmoBoxShodgun_BP_C" (Transformation|GetWorldTransform _arrow) "AlwaysSpawn" 0 0))
    (Transformation|AttachActorToActor _returnvalue_2 self "None" "KeepRelative" "KeepRelative" "KeepRelative" true)
    (Transformation|SetActorRelativeLocation _returnvalue_2 (Variables|/Script/Engine.SceneComponent|GetRelativeLocation _arrow))
    (elif (Math|Integer|InRange(Integer) _returnvalue 26 50)
      (bind _returnvalue_3 (Game|SpawnActorfromClass "/Game/Terrain/Pickups/AmmoChest_BP.AmmoChest_BP_C" (Transformation|GetWorldTransform _arrow_2) "AlwaysSpawn" 0 0))
      (Transformation|AttachActorToActor _returnvalue_3 self "None" "KeepRelative" "KeepRelative" "KeepRelative" true)
      (Transformation|SetActorRelativeLocation _returnvalue_3 (Variables|/Script/Engine.SceneComponent|GetRelativeLocation _arrow_2))
      (elif (Math|Integer|InRange(Integer) _returnvalue 51 75)
        (bind _returnvalue_4 (Game|SpawnActorfromClass "/Game/Terrain/Pickups/Armor+30_BP.Armor+30_BP_C" (Transformation|GetWorldTransform _arrow_3) "AlwaysSpawn" 0 0))
        (Transformation|AttachActorToActor _returnvalue_4 self "None" "KeepRelative" "KeepRelative" "KeepRelative" true)
        (Transformation|SetActorRelativeLocation _returnvalue_4 (Variables|/Script/Engine.SceneComponent|GetRelativeLocation _arrow_3))))))

(event Collision|EventActorBeginOverlap
  (params (OtherActor :type Actor%20Object%20Reference)))

(event EventTick
  (params (DeltaSeconds :type Float%20%28single-precision%29)))

(fn ConstructionScript)
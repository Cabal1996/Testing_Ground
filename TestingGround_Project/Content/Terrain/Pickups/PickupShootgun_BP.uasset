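; Shotgun pickup actor that gives the player a shotgun and a random amount of ammo.
; BeginPlay rolls the ammo amount between configurable min and max values.
; When a player-controlled BP_Character overlaps the collision box, it passes the ammo and Shotgun_BP class with the gun name to the character, calls ItemResive, then destroys itself.
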(event OnComponentBeginOverlap(CollisionBox)
  (params (OverlappedComponent :type Primitive%20Component%20Object%20Reference) (OtherActor :type Actor%20Object%20Reference) (OtherComp :type Primitive%20Component%20Object%20Reference) (OtherBodyIndex :type Integer) (bFromSweep :type Boolean) (SweepResult :type Hit%20Result%20Structure%20%28by%20ref%29))
  (bind _asbp_character (Utilities|Casting|CastToBP_Character OtherActor))
  (if (Pawn|IsPlayerControlled _asbp_character)
    (Class|Mannequin|PickupAmmo _asbp_character (Variables|Default|GetInitialAmmoAmont) (Variables|Default|GetGunName))
    (Class|Mannequin|PickupWeapon _asbp_character "/Game/Weapon/ShotGun_BP.Shotgun_BP_C" (Variables|Default|GetGunName))
    (Default|ItemResive _asbp_character)
    (Actor|DestroyActor)))

(event EventBeginPlay
  (Variables|Default|SetInitialAmmoAmont (Math|Random|RandomIntegerinRange (Variables|Default|GetAmmoAmontMin) (Variables|Default|GetAmmoAmontMax))))

(event Collision|EventActorBeginOverlap
  (params (OtherActor :type Actor%20Object%20Reference)))

(event EventTick
  (params (DeltaSeconds :type Float%20%28single-precision%29)))

(fn ConstructionScript)
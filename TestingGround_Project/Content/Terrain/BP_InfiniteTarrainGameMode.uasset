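; Game mode for an infinite terrain level that builds the ground by chaining BP_Tile actors end to end.
; On BeginPlay it gathers the level's NavMeshBoundsVolumes into a pool, prints debug text and spawns two starting tiles.
; AddTile passes that pool to each new tile, takes its attach location as the next spawn transform and increments Level.
; SpawnTileSet adds a batch of tiles, but its call in the event graph is unwired.
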(event EventBeginPlay
  (bind _outactors (Actor|GetAllActorsOfClass "/Script/NavigationSystem.NavMeshBoundsVolume"))
  (bind _output_get (Variables|Default|SetNavMeshes _outactors))
  (for (_ _array_index) _output_get
    (Development|PrintString (Utilities|String|ToString(Integer) _array_index)))
  (Development|PrintString "Hello")
  (Class|S04TestingGroundGameMode|PopulateBoundsVolumePool (Variables|Default|GetNavMeshes))
  (for _index (range 0 1)
    (CallFunction|AddTile)))

(event EventTick
  (params (DeltaSeconds :type Float%20%28single-precision%29)))

(fn ConstructionScript)

(fn AddTile
  (bind _returnvalue (Game|SpawnActorfromClass "/Game/Terrain/BP_Tile.BP_Tile_C" (Variables|Default|GetNew%20Tile%20Attach%20Loocation) "Undefined" 0 0))
  (Class|Tile|SetPool _returnvalue (Variables|Default|GetNavMeshBoundsVolumePool))
  (bind _attechtransform (Default|GetAttechLocation _returnvalue))
  (Variables|Default|SetNew%20Tile%20Attach%20Loocation _attechtransform)
  (Math|Integer|IncrementInt (Variables|Default|GetLevel)))

(fn SpawnTileSet
  (for _index (range 0 3)
    (CallFunction|AddTile)))
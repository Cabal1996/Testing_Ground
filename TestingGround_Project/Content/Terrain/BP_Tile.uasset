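; BP_Tile is one segment of the infinite terrain, filling itself on BeginPlay with staggered batches of props, rocks and enemies.
; SpawnBoss picks bosses by the game mode's level.
; LockTriggetVolume opens the burning PassBorder once the boss is dead, otherwise shows a boss message, and relocks and calls TileConquered when the player leaves.
; DestroyVolume asks the game mode for another tile, then destroys this one.
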(event OnComponentBeginOverlap(LockTriggetVolume)
  (params (OverlappedComponent :type Primitive%20Component%20Object%20Reference) (OtherActor :type Actor%20Object%20Reference) (OtherComp :type Primitive%20Component%20Object%20Reference) (OtherBodyIndex :type Integer) (bFromSweep :type Boolean) (SweepResult :type Hit%20Result%20Structure%20%28by%20ref%29))
  (bind _returnvalue (Game|GetPlayerCharacter 0))
  (bind _mylevel (Variables|Default|GetMyLevel))
  (bind _returnvalue_2 (== OtherActor _returnvalue))
  (Utilities|FlowControl|Sequence
    (:then_0
      (if (and _returnvalue_2 (Variables|Default|GetBossIsDead))
        (CallFunction|UnLockTile)))
    (:then_1
      (if (Math|Boolean|ANDBoolean (not (Variables|Default|GetBossMesageShown)) (not (Variables|Default|GetBossIsDead)) _returnvalue_2)
        (bind _asplayer_controller_bp (Utilities|Casting|CastToPlayerController_BP (Pawn|GetController _returnvalue)))
        (Default|ShowBossMesage _asplayer_controller_bp)
        (Variables|Default|SetBossMesageShown true)
        (if (not (Collision|IsOverlappingActor (Variables|Default|GetLockTriggetVolume) (Variables|Default|GetBoss) :!class /Script/Engine.PrimitiveComponent))
          (CallFunction|SpawnBoss "/Game/Character/BP_Character_Child_YellowBoss.BP_Character_Child_YellowBoss_C" _mylevel 4)
          (CallFunction|SpawnBoss "/Game/Character/BP_Character_Child_RedBoss.BP_Character_Child_RedBoss_C" _mylevel 8)
          (CallFunction|SpawnBoss "/Game/Character/BP_Character_Child_BlueBoss.BP_Character_Child_BlueBoss_C" _mylevel 12))))))

(event OnComponentEndOverlap(LockTriggetVolume)
  (params (OverlappedComponent :type Primitive%20Component%20Object%20Reference) (OtherActor :type Actor%20Object%20Reference) (OtherComp :type Primitive%20Component%20Object%20Reference) (OtherBodyIndex :type Integer))
  (if (== OtherActor (Game|GetPlayerCharacter 0))
    (Utilities|FlowControl|Sequence
      (:then_0
        (CallFunction|LockTile))
      (:then_1
        (Class|Tile|TileConquered)))))

(event OnComponentBeginOverlap(DestroyVolume)
  (params (OverlappedComponent :type Primitive%20Component%20Object%20Reference) (OtherActor :type Actor%20Object%20Reference) (OtherComp :type Primitive%20Component%20Object%20Reference) (OtherBodyIndex :type Integer) (bFromSweep :type Boolean) (SweepResult :type Hit%20Result%20Structure%20%28by%20ref%29))
  (if (== OtherActor (Game|GetPlayerCharacter 0))
    (Default|AddTile (Variables|Default|GetGameMode))
    (Class|Tile|DestroyTile)
    (Actor|DestroyActor)))

(event Custom|Burning
  (bind _burnvalue (Timeline|Timeline_0 PlayFromStart)
    (:Update
      (Rendering|Material|SetScalarParameterValueonMaterials (Variables|Default|GetPassBorder) "Burn" _burnvalue))))

(event Custom|UnBurnung
  (bind _burnvalue (Timeline|Timeline_0 ReverseFromEnd)
    (:Update
      (Rendering|Material|SetScalarParameterValueonMaterials (Variables|Default|GetPassBorder) "Burn" _burnvalue))))

(event EventBeginPlay
  (bind _asbp_infinite_tarrain_game_mode (Utilities|Casting|CastToBP_InfiniteTarrainGameMode (Game|GetGameMode)))
  (bind _output_get (Variables|Default|SetGameMode _asbp_infinite_tarrain_game_mode))
  (Variables|Default|SetMyLevel (Variables|/Game/Terrain/BP_InfiniteTarrainGameMode.BP_InfiniteTarrainGameMode_C|GetLevel _output_get))
  (CallFunction|SpawnBoss "/Game/Character/BP_Character_Child_YellowBoss.BP_Character_Child_YellowBoss_C" (Variables|Default|GetMyLevel) 4)
  (CallFunction|SpawnBoss "/Game/Character/BP_Character_Child_RedBoss.BP_Character_Child_RedBoss_C" (Variables|Default|GetMyLevel) 8)
  (CallFunction|SpawnBoss "/Game/Character/BP_Character_Child_BlueBoss.BP_Character_Child_BlueBoss_C" (Variables|Default|GetMyLevel) 12)
  (Class|Tile|PlaceActors "/Game/Terrain/Props/BP_Container.BP_Container_C" 1 3 5.1e+02 1.0 1.0)
  (Utilities|FlowControl|Delay (Variables|Default|GetSpawnDelay))
  (Class|Tile|PlaceActors "/Game/Terrain/Props/BP_ArmyBox.BP_ArmyBox_C" 2 4 1e+02 1.0 1.0)
  (Utilities|FlowControl|Delay (Variables|Default|GetSpawnDelay))
  (Class|Tile|PlaceActors "/Game/Terrain/Props/BP_Canister.BP_Canister_C" 1 7 5e+01 1.0 1.0)
  (Utilities|FlowControl|Delay (Variables|Default|GetSpawnDelay))
  (Class|Tile|PlaceActors "/Game/Terrain/Props/BP_Rock_S.BP_Rock_S_C" 0 4 1.5e+02 1.0 5.0)
  (Utilities|FlowControl|Delay (Variables|Default|GetSpawnDelay))
  (Class|Tile|PlaceActors "/Game/Terrain/Props/BP_Rock_M.BP_Rock_M_C" 0 4 2.5e+02 1.0 5.0)
  (Utilities|FlowControl|Delay (Variables|Default|GetSpawnDelay))
  (Class|Tile|PlaceActors "/Game/Terrain/Props/BP_Rock_L.BP_Rock_L_C" 0 4 2.5e+02 1.0 5.0)
  (Utilities|FlowControl|Delay (Variables|Default|GetSpawnDelay))
  (Class|Tile|PlaceActors "/Game/Terrain/Props/BP_SackWall.BP_SackWall_C" 0 2 5e+02 1.0 1.0)
  (Utilities|FlowControl|Delay (Variables|Default|GetSpawnDelay))
  (Class|Tile|PlaceAIPawns "/Game/Character/BP_Character.BP_Character_C" (Variables|Default|GetMaxEnemys) (Variables|Default|GetMaxEnemys) 1e+02))

(event Collision|EventActorBeginOverlap
  (params (OtherActor :type Actor%20Object%20Reference)))

(event EventTick
  (params (DeltaSeconds :type Float%20%28single-precision%29)))

(fn ConstructionScript)

(fn GetAttechLocation
  (return (Transformation|GetWorldTransform (Variables|Default|GetArrow))))

(fn LockTile
  (Collision|SetCollisionEnabled (Variables|Default|GetPassBorder) "QueryAndPhysics")
  (CallFunction|UnBurnung))

(fn UnLockTile
  (Collision|SetCollisionEnabled (Variables|Default|GetPassBorder) "NoCollision")
  (CallFunction|Burning))

(fn SpawnBoss
  (params (Spawn :type Mannequin%20Class%20Reference) (CurrentLevel :type Integer) (SpawnLevel :type Integer))
  (if (== CurrentLevel SpawnLevel)
    (Class|Tile|PlaceAIPawns Spawn 1 1 1e+02)
    (Variables|Default|SetBossIsDead false)
    (elif (>= CurrentLevel (Variables|Default|GetLastLevel))
      (Class|Tile|PlaceAIPawns Spawn 0 1 1e+02))))
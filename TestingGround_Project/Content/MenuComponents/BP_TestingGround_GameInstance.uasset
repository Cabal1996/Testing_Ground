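; BP_TestingGround_GameInstance is a Game Instance that exposes the game's video settings through a getter and a setter.
; GetVideoOption reads anti-aliasing, post-processing, texture, shadow, view distance and visual effect quality, plus VSync, from GameUserSettings.
; SetVideoOptions writes the same values back in sequence, then calls ApplySettings to commit them.
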(fn GetVideoOption
  (bind _returnvalue (Settings|GetGameUserSettings))
  (return (Class|GameUserSettings|GetAntiAliasingQuality _returnvalue) (Class|GameUserSettings|GetPostProcessingQuality _returnvalue) (Class|GameUserSettings|GetTextureQuality _returnvalue) (Settings|GetShadowQuality _returnvalue) (Class|GameUserSettings|GetViewDistanceQuality _returnvalue) (Settings|GetVisualEffectQuality _returnvalue) (Class|GameUserSettings|IsVSyncEnabled _returnvalue)))

(fn SetVideoOptions
  (params (Anti-Aliasing :type Integer) (Post%20Processing :type Integer) (Texture%20Quality :type Integer) (Shadow%20Quality :type Integer) (View%20Distance%20Quality :type Integer) (Visual%20Effect%20Quality :type Integer) (VSync%20Enabled :type Boolean))
  (bind _returnvalue (Settings|GetGameUserSettings))
  (Utilities|FlowControl|Sequence
    (:then_0
      (Class|GameUserSettings|SetAntiAliasingQuality _returnvalue Anti-Aliasing))
    (:then_1
      (Class|GameUserSettings|SetPostProcessingQuality _returnvalue Post%20Processing))
    (:then_2
      (Class|GameUserSettings|SetTextureQuality _returnvalue Texture%20Quality))
    (:then_3
      (Class|GameUserSettings|SetShadowQuality _returnvalue Shadow%20Quality))
    (:then_4
      (Class|GameUserSettings|SetViewDistanceQuality _returnvalue View%20Distance%20Quality))
    (:then_5
      (Class|GameUserSettings|SetVisualEffectQuality _returnvalue Visual%20Effect%20Quality))
    (:then_6
      (Class|GameUserSettings|SetVSyncEnabled _returnvalue VSync%20Enabled))
    (:then_7
      (Class|GameUserSettings|ApplySettings _returnvalue true))))
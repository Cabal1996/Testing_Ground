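; BP_Character_Child_YellowBoss is a child character Blueprint for the yellow boss tied to a BP_Tile.
; Shortly after BeginPlay it casts its attach parent to BP_Tile and registers itself as that tile's Boss.
; On death it unlocks the tile once, guarded by the tile's BossIsDead flag.
; Its DropPickUp event spawns a shotgun pickup at its transform if WasAlive is set.
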(event EventBeginPlay
  (|CallParentFunction)
  (Utilities|FlowControl|Delay 0.5)
  (bind _asbp_tile (Utilities|Casting|CastToBP_Tile (Actor|GetAttachParentActor)))
  (Variables|/Game/Terrain/BP_Tile.BP_Tile_C|SetBoss _asbp_tile self))

(event Collision|EventActorBeginOverlap
  (params (OtherActor :type Actor%20Object%20Reference)))

(event EventTick
  (params (DeltaSeconds :type Float%20%28single-precision%29))
  (|CallParentFunction DeltaSeconds) ; This node is disabled and will not be called.\nDrag off pins to build functionality.
)

(event EventDropPickUp
  (if (Variables|Default|GetWasAlive)
    (Game|SpawnActorfromClass "/Game/Terrain/Pickups/PickupShootgun_BP.PickupShootgun_BP_C" (Transformation|GetActorTransform) "Undefined" 0 0)))

(event EventOnDeath
  (bind _asbp_tile (Utilities|Casting|CastToBP_Tile (Actor|GetAttachParentActor)))
  (if (not (Variables|/Game/Terrain/BP_Tile.BP_Tile_C|GetBossIsDead _asbp_tile))
    (Default|UnLockTile _asbp_tile)
    (Variables|/Game/Terrain/BP_Tile.BP_Tile_C|SetBossIsDead _asbp_tile true)))

(fn ConstructionScript
  (|CallParentFunction))
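; AI controller for guard NPCs that runs the GuardBehaviour tree on the PatrolData blackboard and keeps a reference to its possessed BP_Character.
; AI perception ignores actors tagged "Enemy"; any other sensed actor is written to the EnemyKey blackboard entry and becomes the focus.
; When that perception reports a failed sense, it clears the key and focus and tells the pawn to release the trigger.
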(event OnTargetPerceptionUpdated(AIPerception)
  (params (Actor :type Actor%20Object%20Reference) (Stimulus :type AI%20Stimulus%20Structure))
  (bind _enemykey (Variables|Default|GetEnemyKey))
  (bind _blackboardcomp (Variables|Default|GetBlackBoardComp))
  (if (not (Actor|ActorHasTag Actor "Enemy"))
    (if (.bSuccessfullySensed (Utilities|Struct|BreakAIStimulus Stimulus))
      (AI|Components|Blackboard|SetValueasObject _blackboardcomp _enemykey Actor)
      (AI|SetFocus Actor)
      (else
        (AI|Components|Blackboard|ClearValue _blackboardcomp _enemykey)
        (AI|ClearFocus)
        (Class|Mannequin|ReleaseTrigger (Variables|Default|GetControlledPawnAsNPC))))))

(event EventBeginPlay
  (bind _blackboardcomponent (Class|AIController|UseBlackboard "/Game/Character/AI/PatrolData.PatrolData"))
  (AI|RunBehaviorTree "/Game/Character/AI/GuardBehaviour.GuardBehaviour")
  (Variables|Default|SetBlackBoardComp _blackboardcomponent))

(event EventOnPossess
  (params (PossessedPawn :type Pawn%20Object%20Reference))
  (bind _asbp_character (Utilities|Casting|CastToBP_Character PossessedPawn))
  (Variables|Default|SetControlledPawnAsNPC _asbp_character))

(fn ConstructionScript)
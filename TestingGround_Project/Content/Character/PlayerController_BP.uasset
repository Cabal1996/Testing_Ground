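; Player controller that owns the HUD and pause menu and manages the player's sound and mouse settings.
; BeginPlay creates both widgets and loads or creates the save game for master volume; Quit or P toggles the menu, pausing on open and passing it current graphics settings.
; Tick projects a muzzle trace onto the right-click-toggled adaptive crosshair and times the damage-dealt indicator.
; Sensitivity setters rewrite Turn/LookUp axis mapping scales; G prints saved results.
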(event Custom|OnPawnDeath)

(event EventBeginPlay
  (bind _self self)
  (bind _returnvalue (UserInterface|CreateWidget "/Game/UI/Menu.Menu_C" self))
  (bind _output_get (Variables|Default|SetMenuWidget _returnvalue))
  (Default|SetPlayerController _output_get _self)
  (bind _asbp_character (Utilities|Casting|CastToBP_Character (Pawn|GetControlledPawn _self)))
  (Default|SetPlayer _output_get _asbp_character)
  (bind _returnvalue_2 (UserInterface|CreateWidget "/Game/UI/MainUI.MainUI_C" self))
  (UserInterface|Viewport|AddtoPlayerScreen _returnvalue_2)
  (Variables|Default|SetMainUIWidget _returnvalue_2)
  (bind _asbp_character_2 (Utilities|Casting|CastToBP_Character (Pawn|GetControlledPawn)))
  (Variables|Default|SetControlledCharacter _asbp_character_2)
  (Utilities|FlowControl|Delay 0.2)
  (Class|GameplayStatics|SetBaseSoundMix "/Game/Character/NewSoundMix.NewSoundMix")
  (bind _returnvalue_3 (SaveGame|DoesSaveGameExist "MainSave"))
  (if _returnvalue_3
    (bind _returnvalue_4 (SaveGame|LoadGamefromSlot "MainSave"))
    (bind _asbp_save_game (Utilities|Casting|CastToBP_SaveGame _returnvalue_4))
    (Variables|Default|SetMainSaveGame _asbp_save_game)
    (Setter|SetSoundVolume (Variables|/Game/MenuComponents/BP_SaveGame.BP_SaveGame_C|GetSoundVolume _asbp_save_game))
    (else
      (bind _returnvalue_5 (SaveGame|CreateSaveGameObject "/Game/MenuComponents/BP_SaveGame.BP_SaveGame_C"))
      (Variables|Default|SetMainSaveGame _returnvalue_5)
      (Setter|SetSoundVolume (Variables|Default|GetSoundVolume)))))

(event EventTick
  (params (DeltaSeconds :type Float%20%28single-precision%29))
  (CallFunction|AdaptiveCrosshairMovement 0.0)
  (CallFunction|DamageIndicatorControl DeltaSeconds))

(event Input|ActionEvents|InputActionQuit
  (params (Key :type Key%20Structure))
  (bind _menuwidget (Variables|Default|GetMenuWidget))
  (:Pressed
    (if (Variables|Default|GetMenuIsOpen)
      (Widget|RemovefromParent (Variables|Default|GetMenuWidget))
      (Variables|Default|SetMenuIsOpen false)
      (Variables|Default|SetbShowMouseCursor false)
      (Input|SetInputModeGameOnly self)
      (else
        (UserInterface|Viewport|AddtoViewport (Variables|Default|GetMenuWidget) 0)
        (Variables|Default|SetMenuIsOpen true)
        (Variables|Default|SetbShowMouseCursor true)
        (Input|SetInputModeUIOnly self (Variables|Default|GetMenuWidget) "DoNotLock")
        (bind _returnvalue (Settings|GetGameUserSettings))
        (Default|GetAntiAliasing _menuwidget (Class|GameUserSettings|GetAntiAliasingQuality _returnvalue))
        (Default|GetPostProcessing _menuwidget (Class|GameUserSettings|GetPostProcessingQuality _returnvalue))
        (Default|GetTextureQuality _menuwidget (Class|GameUserSettings|GetTextureQuality _returnvalue))
        (Default|ShadowQuality _menuwidget (Settings|GetShadowQuality _returnvalue))
        (Default|GetViewDistance _menuwidget (Class|GameUserSettings|GetViewDistanceQuality _returnvalue))
        (Default|GetVisualEffect _menuwidget (Settings|GetVisualEffectQuality _returnvalue))
        (Default|GetV-Sync _menuwidget (Class|GameUserSettings|IsVSyncEnabled _returnvalue))
        (Game|SetGamePaused true)))))

(event Input|MouseEvents|RightMouseButton
  (params (Key :type Key%20Structure))
  (:Pressed
    (if (Variables|Default|GetIsAdaptivCrosshair)
      (Variables|Default|SetIsAdaptivCrosshair false)
      (else
        (Variables|Default|SetIsAdaptivCrosshair true)))))

(event Input|KeyboardEvents|G
  (params (Key :type Key%20Structure))
  (:Pressed
    (for _array_element (Variables|/Game/MenuComponents/BP_SaveGame.BP_SaveGame_C|GetgameResaults (Variables|Default|GetMainSaveGame))
      (Development|PrintString (Utilities|String|Append (Utilities|String|ToString(Name) (.PlayerName (Utilities|Struct|BreakGameResult _array_element))) " " (Utilities|String|ToString(Integer) (.Score (Utilities|Struct|BreakGameResult _array_element))) " " (Class|KismetStringLibrary|TimeSecondstoString (.Time (Utilities|Struct|BreakGameResult _array_element))))))))

(event Input|KeyboardEvents|P
  (params (Key :type Key%20Structure))
  (bind _menuwidget (Variables|Default|GetMenuWidget))
  (:Pressed
    (if (Variables|Default|GetMenuIsOpen)
      (Widget|RemovefromParent (Variables|Default|GetMenuWidget))
      (Variables|Default|SetMenuIsOpen false)
      (Variables|Default|SetbShowMouseCursor false)
      (Input|SetInputModeGameOnly self)
      (else
        (UserInterface|Viewport|AddtoViewport (Variables|Default|GetMenuWidget) 0)
        (Variables|Default|SetMenuIsOpen true)
        (Variables|Default|SetbShowMouseCursor true)
        (Input|SetInputModeUIOnly self (Variables|Default|GetMenuWidget) "DoNotLock")
        (bind _returnvalue (Settings|GetGameUserSettings))
        (Default|GetAntiAliasing _menuwidget (Class|GameUserSettings|GetAntiAliasingQuality _returnvalue))
        (Default|GetPostProcessing _menuwidget (Class|GameUserSettings|GetPostProcessingQuality _returnvalue))
        (Default|GetTextureQuality _menuwidget (Class|GameUserSettings|GetTextureQuality _returnvalue))
        (Default|ShadowQuality _menuwidget (Settings|GetShadowQuality _returnvalue))
        (Default|GetViewDistance _menuwidget (Class|GameUserSettings|GetViewDistanceQuality _returnvalue))
        (Default|GetVisualEffect _menuwidget (Settings|GetVisualEffectQuality _returnvalue))
        (Default|GetV-Sync _menuwidget (Class|GameUserSettings|IsVSyncEnabled _returnvalue))
        (Game|SetGamePaused true)))))

(fn ConstructionScript)

(fn SetXAxisSensetivity
  (params (New%20Sensativity%20Value :type Float%20%28single-precision%29))
  (bind _returnvalue (Class|InputSettings|GetInputSettings))
  (for _array_element (Class|InputSettings|GetAxisMappingbyName _returnvalue "Turn")
    (bind _output_get (Variables|Default|SetXAxisKeyMapping _array_element))
    (Class|InputSettings|RemoveAxisMapping _returnvalue _array_element true)
    (Class|InputSettings|AddAxisMapping _returnvalue (Utilities|Struct|MakeInputAxisKeyMapping (.AxisName (Utilities|Struct|BreakInputAxisKeyMapping _output_get)) (Math|Float|Clamp(Float) New%20Sensativity%20Value 0.01) (.Key (Utilities|Struct|BreakInputAxisKeyMapping _output_get))) true)
    (Class|InputSettings|SaveKeyMappings _returnvalue)))

(fn SetYAxisSensetivity
  (params (New%20Sensativity%20Value :type Float%20%28single-precision%29))
  (bind _returnvalue (Class|InputSettings|GetInputSettings))
  (for _array_element (Class|InputSettings|GetAxisMappingbyName _returnvalue "LookUp")
    (bind _output_get (Variables|Default|SetYAxisKeyMapping _array_element))
    (Class|InputSettings|RemoveAxisMapping _returnvalue _array_element true)
    (Class|InputSettings|AddAxisMapping _returnvalue (Utilities|Struct|MakeInputAxisKeyMapping (.AxisName (Utilities|Struct|BreakInputAxisKeyMapping _output_get)) (Math|Float|Clamp(Float) (* New%20Sensativity%20Value -1.0) -1.0 -0.01) (.Key (Utilities|Struct|BreakInputAxisKeyMapping _output_get))) true)
    (Class|InputSettings|SaveKeyMappings _returnvalue)))

(fn GetXAxisSensetivity
  (for _array_element (Class|InputSettings|GetAxisMappingbyName (Class|InputSettings|GetInputSettings) "Turn")
    (return (.Scale (Utilities|Struct|BreakInputAxisKeyMapping _array_element)))))

(fn GetYAxisSensetivity
  (for _array_element (Class|InputSettings|GetAxisMappingbyName (Class|InputSettings|GetInputSettings) "LookUp")
    (return (* (.Scale (Utilities|Struct|BreakInputAxisKeyMapping _array_element)) -1.0))))

(fn ShowBossMesage
  (Default|ShowBossMesage (Variables|Default|GetMainUIWidget)))

(fn ResiveDamageNPC
  (Variables|Default|SetDamageDone true))

(fn AdaptiveCrosshairMovement
  (params (DeltaTime :type Float%20%28single-precision%29))
  (bind _controlledcharacter (Variables|Default|GetControlledCharacter))
  (bind _returnvalue (Class|Mannequin|GetGun _controlledcharacter))
  (bind _returnvalue_2 (Class|Gun|GetMuzzleLocation _returnvalue))
  (bind _returnvalue_3 (Transformation|GetWorldLocation _returnvalue_2))
  (if (Variables|Default|GetIsAdaptivCrosshair)
    (bind (_outhit _returnvalue_4) (Collision|LineTraceByChannel _returnvalue_3 (+ _returnvalue_3 (* (Math|Vector|GetForwardVector _returnvalue_2) 1e+05)) "TraceTypeQuery1" false 0 "None" false))
    (if _returnvalue_4
      (Default|SetCrosshairPosition (Variables|Default|GetMainUIWidget) (.ScreenPosition (Class|WidgetLayoutLibrary|ProjectWorldLocationtoWidgetPosition self (.ImpactPoint (Collision|BreakHitResult _outhit))))))))

(fn DamageIndicatorControl
  (params (DeltaTime :type Float%20%28single-precision%29))
  (if (Variables|Default|GetDamageDone)
    (Variables|/Game/UI/MainUI.MainUI_C|SetIsVisibleDmgIndicator (Variables|Default|GetMainUIWidget) true)
    (Variables|Default|SetLastApear (+ (Variables|Default|GetLastApear) DeltaTime))
    (if (> (Variables|Default|GetLastApear) (Variables|Default|GetDelay))
      (Variables|/Game/UI/MainUI.MainUI_C|SetIsVisibleDmgIndicator (Variables|Default|GetMainUIWidget) false)
      (Variables|Default|SetLastApear 0.0)
      (Variables|Default|SetDamageDone false))))

(fn GetSoundVolume
  (return (Variables|Default|GetSoundVolume)))

(fn SetSoundVolume
  (params (NewSoundVolume :type Float%20%28single-precision%29))
  (bind _mainsavegame (Variables|Default|GetMainSaveGame))
  (bind _output_get (Variables|Default|SetSoundVolume (Math|Float|Clamp(Float) NewSoundVolume 0.01)))
  (Audio|SetSoundMixClassOverride "/Game/Character/NewSoundMix.NewSoundMix" "/Engine/EngineSounds/Master.Master" _output_get 1.0 0.0 true)
  (Utilities|IsValid _mainsavegame
    (:Is%20Valid
      (Variables|/Game/MenuComponents/BP_SaveGame.BP_SaveGame_C|SetSoundVolume _mainsavegame (Variables|Default|GetSoundVolume))
      (bind _returnvalue (SaveGame|SaveGametoSlot _mainsavegame "MainSave"))
      (if (not _returnvalue)
        (Development|PrintString "Saving error")))))